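; CheeringCharacter_BP is a tower-level character that loops a cheer animation on its skeletal mesh as soon as play begins.
; Cheer sets and loops the cheer animation, while Show makes the mesh visible and switches it to a looping idle.
; Hide turns off mesh visibility, but its only call in the event graph is disconnected and never runs.
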(event EventBeginPlay
  (CallFunction|Cheer))

(event Collision|EventActorBeginOverlap
  (params (OtherActor :type Actor%20Object%20Reference)))

(event EventTick
  (params (DeltaSeconds :type Float%20%28single-precision%29)))

(fn ConstructionScript)

(fn Cheer
  (bind _sk_character (Variables|Default|GetSK_Character))
  (Components|Animation|SetAnimation _sk_character "/Game/characters/common/Animations/AN_cheer.AN_cheer")
  (Components|Animation|PlayAnimation _sk_character "/Game/characters/common/Animations/AN_cheer.AN_cheer" true))

(fn Show
  (bind _sk_character (Variables|Default|GetSK_Character))
  (Rendering|SetVisibility (Variables|Default|GetSK_Character) true false)
  (Components|Animation|SetAnimation _sk_character "/Game/characters/hero/animations/AN_idle.AN_idle")
  (Components|Animation|PlayAnimation _sk_character "/Game/characters/hero/animations/AN_idle.AN_idle" true))

(fn Hide
  (Rendering|SetVisibility (Variables|Default|GetSK_Character) false false))