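; Controller actor for the tower level that manages four colored cheering characters: Red, Green, Blue and Yellow.
; It hides all four on BeginPlay and exposes a separate show function for each color.
; StartCheer triggers the cheer on all four in sequence, casting each reference to CheeringCharacter_BP.
; In HideAll and StartCheer a failed cast stops the remaining characters from being processed.
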(event EventBeginPlay
  (CallFunction|HideAll))

(event Collision|EventActorBeginOverlap
  (params (OtherActor :type Actor%20Object%20Reference)))

(event EventTick
  (params (DeltaSeconds :type Float%20%28single-precision%29)))

(fn ConstructionScript)

(fn HideAll
  (bind _ascheering_character_bp (Utilities|Casting|CastToCheeringCharacter_BP (Variables|Default|GetRed)))
  (Default|Hide _ascheering_character_bp)
  (bind _ascheering_character_bp_2 (Utilities|Casting|CastToCheeringCharacter_BP (Variables|Default|GetGreen)))
  (Default|Hide _ascheering_character_bp_2)
  (bind _ascheering_character_bp_3 (Utilities|Casting|CastToCheeringCharacter_BP (Variables|Default|GetBlue)))
  (Default|Hide _ascheering_character_bp_3)
  (bind _ascheering_character_bp_4 (Utilities|Casting|CastToCheeringCharacter_BP (Variables|Default|GetYellow)))
  (Default|Hide _ascheering_character_bp_4))

(fn ShowRed
  (bind _ascheering_character_bp (Utilities|Casting|CastToCheeringCharacter_BP (Variables|Default|GetRed)))
  (Default|Show _ascheering_character_bp))

(fn ShowBlue
  (bind _ascheering_character_bp (Utilities|Casting|CastToCheeringCharacter_BP (Variables|Default|GetBlue)))
  (Default|Show _ascheering_character_bp))

(fn ShowGreen
  (bind _ascheering_character_bp (Utilities|Casting|CastToCheeringCharacter_BP (Variables|Default|GetGreen)))
  (Default|Show _ascheering_character_bp))

(fn ShowYellow
  (bind _ascheering_character_bp (Utilities|Casting|CastToCheeringCharacter_BP (Variables|Default|GetYellow)))
  (Default|Show _ascheering_character_bp))

(fn StartCheer
  (bind _ascheering_character_bp (Utilities|Casting|CastToCheeringCharacter_BP (Variables|Default|GetRed)))
  (Default|Cheer _ascheering_character_bp)
  (bind _ascheering_character_bp_2 (Utilities|Casting|CastToCheeringCharacter_BP (Variables|Default|GetGreen)))
  (Default|Cheer _ascheering_character_bp_2)
  (bind _ascheering_character_bp_3 (Utilities|Casting|CastToCheeringCharacter_BP (Variables|Default|GetBlue)))
  (Default|Cheer _ascheering_character_bp_3)
  (bind _ascheering_character_bp_4 (Utilities|Casting|CastToCheeringCharacter_BP (Variables|Default|GetYellow)))
  (Default|Cheer _ascheering_character_bp_4))