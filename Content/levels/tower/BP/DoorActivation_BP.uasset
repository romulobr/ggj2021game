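; Tower level trigger that breaks the wall door apart when the tower ball overlaps it, framed by a short camera cutaway.
; The overlapping actor is matched by display name, then the hero character switches to the internal tower camera.
; After a delay, the door and crack wall pieces start simulating physics.
; After a second delay, the hero returns to the follow camera.
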(event EventBeginPlay)

(event Collision|EventActorBeginOverlap
  (params (OtherActor :type Actor%20Object%20Reference))
  (if (Utilities|Enum|Equal(Enum) (Utilities|GetDisplayName OtherActor) "SM_TowerBall")
    (bind _ashero_character_bp (Utilities|Casting|CastToheroCharacter_BP (Game|GetPlayerCharacter 0)))
    (Default|ChangeCameratoInternalTowerCamera _ashero_character_bp)
    (Utilities|FlowControl|Delay 3.0)
    (Physics|SetSimulatePhysics (Variables|Default|GetSM_TowerWallDoorPiece3) true)
    (Utilities|FlowControl|Delay 3.0)
    (Default|ChangeCameratoFollowCamera _ashero_character_bp)))

(event EventTick
  (params (DeltaSeconds :type Float%20%28single-precision%29)))

(fn ConstructionScript)