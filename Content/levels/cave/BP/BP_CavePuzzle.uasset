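; Cave level puzzle that opens a prison cell once all four trigger boxes are occupied by something other than the player.
; Each box plays a hit sound and sets its flag on overlap, then clears it on exit.
; Tick polls the flags, switches the hero to a puzzle-end camera, waits briefly, destroys the cell, restores the follow camera and marks the puzzle finished.
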(event OnComponentBeginOverlap(Box1)
  (params (OverlappedComponent :type Primitive%20Component%20Object%20Reference) (OtherActor :type Actor%20Object%20Reference) (OtherComp :type Primitive%20Component%20Object%20Reference) (OtherBodyIndex :type Integer) (bFromSweep :type Boolean) (SweepResult :type Hit%20Result%20Structure%20%28by%20ref%29))
  (if (!= OtherActor (Game|GetPlayerCharacter 0))
    (Audio|PlaySound2D "/Game/levels/MusicSFX/SFX/Tower_-_SFx_-_Esfera_Atigindo_o_Alvo_2.Tower_-_SFx_-_Esfera_Atigindo_o_Alvo_2" 1.0 1.0 0.0 0 0)
    (Variables|Default|SetIsTrigger1Activated true)))

(event OnComponentEndOverlap(Box1)
  (params (OverlappedComponent :type Primitive%20Component%20Object%20Reference) (OtherActor :type Actor%20Object%20Reference) (OtherComp :type Primitive%20Component%20Object%20Reference) (OtherBodyIndex :type Integer))
  (if (!= OtherActor (Game|GetPlayerCharacter 0))
    (Variables|Default|SetIsTrigger1Activated false)))

(event OnComponentBeginOverlap(Box2)
  (params (OverlappedComponent :type Primitive%20Component%20Object%20Reference) (OtherActor :type Actor%20Object%20Reference) (OtherComp :type Primitive%20Component%20Object%20Reference) (OtherBodyIndex :type Integer) (bFromSweep :type Boolean) (SweepResult :type Hit%20Result%20Structure%20%28by%20ref%29))
  (if (!= OtherActor (Game|GetPlayerCharacter 0))
    (Audio|PlaySound2D "/Game/levels/MusicSFX/SFX/Tower_-_SFx_-_Esfera_Atigindo_o_Alvo_2.Tower_-_SFx_-_Esfera_Atigindo_o_Alvo_2" 1.0 1.0 0.0 0 0)
    (Variables|Default|SetIsTrigger2Activated true)))

(event OnComponentEndOverlap(Box2)
  (params (OverlappedComponent :type Primitive%20Component%20Object%20Reference) (OtherActor :type Actor%20Object%20Reference) (OtherComp :type Primitive%20Component%20Object%20Reference) (OtherBodyIndex :type Integer))
  (if (!= OtherActor (Game|GetPlayerCharacter 0))
    (Variables|Default|SetIsTrigger2Activated false)))

(event OnComponentBeginOverlap(Box3)
  (params (OverlappedComponent :type Primitive%20Component%20Object%20Reference) (OtherActor :type Actor%20Object%20Reference) (OtherComp :type Primitive%20Component%20Object%20Reference) (OtherBodyIndex :type Integer) (bFromSweep :type Boolean) (SweepResult :type Hit%20Result%20Structure%20%28by%20ref%29))
  (if (!= OtherActor (Game|GetPlayerCharacter 0))
    (Audio|PlaySound2D "/Game/levels/MusicSFX/SFX/Tower_-_SFx_-_Esfera_Atigindo_o_Alvo_2.Tower_-_SFx_-_Esfera_Atigindo_o_Alvo_2" 1.0 1.0 0.0 0 0)
    (Variables|Default|SetIsTrigger3Activated true)))

(event OnComponentEndOverlap(Box3)
  (params (OverlappedComponent :type Primitive%20Component%20Object%20Reference) (OtherActor :type Actor%20Object%20Reference) (OtherComp :type Primitive%20Component%20Object%20Reference) (OtherBodyIndex :type Integer))
  (if (!= OtherActor (Game|GetPlayerCharacter 0))
    (Variables|Default|SetIsTrigger3Activated false)))

(event OnComponentBeginOverlap(Box4)
  (params (OverlappedComponent :type Primitive%20Component%20Object%20Reference) (OtherActor :type Actor%20Object%20Reference) (OtherComp :type Primitive%20Component%20Object%20Reference) (OtherBodyIndex :type Integer) (bFromSweep :type Boolean) (SweepResult :type Hit%20Result%20Structure%20%28by%20ref%29))
  (if (!= OtherActor (Game|GetPlayerCharacter 0))
    (Audio|PlaySound2D "/Game/levels/MusicSFX/SFX/Tower_-_SFx_-_Esfera_Atigindo_o_Alvo_2.Tower_-_SFx_-_Esfera_Atigindo_o_Alvo_2" 1.0 1.0 0.0 0 0)
    (Variables|Default|SetIsTrigger4Activated true)))

(event OnComponentEndOverlap(Box4)
  (params (OverlappedComponent :type Primitive%20Component%20Object%20Reference) (OtherActor :type Actor%20Object%20Reference) (OtherComp :type Primitive%20Component%20Object%20Reference) (OtherBodyIndex :type Integer))
  (if (!= OtherActor (Game|GetPlayerCharacter 0))
    (Variables|Default|SetIsTrigger4Activated false)))

(event EventBeginPlay)

(event Collision|EventActorBeginOverlap
  (params (OtherActor :type Actor%20Object%20Reference)))

(event EventTick
  (params (DeltaSeconds :type Float%20%28single-precision%29))
  (bind _response (CallFunction|AllTriggersActivated))
  (if (and _response (not (Variables|Default|GetFinished)))
    (bind _ashero_character_bp (Utilities|Casting|CastToheroCharacter_BP (Game|GetPlayerCharacter 0)))
    (Default|ChangeCameratoCavePuzzleEnd _ashero_character_bp)
    (Utilities|FlowControl|Delay 5.0)
    (Actor|DestroyActor (Variables|Default|GetPrisonCell))
    (Default|ChangeCameratoFollowCamera _ashero_character_bp)
    (Variables|Default|SetFinished true)))

(fn ConstructionScript)

(fn AllTriggersActivated
  (return (and (and (Variables|Default|GetIsTrigger1Activated) (Variables|Default|GetIsTrigger2Activated)) (and (Variables|Default|GetIsTrigger3Activated) (Variables|Default|GetIsTrigger4Activated)))))