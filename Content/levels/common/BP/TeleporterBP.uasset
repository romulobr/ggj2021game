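; Teleporter actor that moves the player character to a Destination actor's location after a cinematic camera transition.
; On player overlap, TransitionCameraName selects one of the hero's Mountain, Maze, Forest or Cave teleport cameras, falling back to the external tower camera.
; A teleport sound plays, delayed for named transitions, then timed delays sequence the location change and the return to the follow camera.
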(event EventBeginPlay)

(event Collision|EventActorBeginOverlap
  (params (OtherActor :type Actor%20Object%20Reference))
  (bind _returnvalue (Game|GetPlayerCharacter 0))
  (if (== OtherActor _returnvalue)
    (bind _ashero_character_bp (Utilities|Casting|CastToheroCharacter_BP _returnvalue))
    (if (Utilities|Enum|Equal(Enum) (Variables|Default|GetTransitionCameraName) "Mountain")
      (Default|ChangeCameratoMountainTeleport _ashero_character_bp)
      (Utilities|FlowControl|Delay 1.5 :!label _label)
      (Audio|PlaySound2D "/Game/levels/MusicSFX/SFX/The_Tower_-_SFx__Teleporte_.The_Tower_-_SFx__Teleporte_" 1.0 1.0 0.0 0 0)
      (elif (Utilities|Enum|Equal(Enum) (Variables|Default|GetTransitionCameraName) "Maze")
        (Default|ChangeCameratoMazeTeleport _ashero_character_bp)
        (goto _label)
        (elif (Utilities|Enum|Equal(Enum) (Variables|Default|GetTransitionCameraName) "Forest")
          (Default|ChangeCameratoForestTeleport _ashero_character_bp)
          (goto _label)
          (elif (Utilities|Enum|Equal(Enum) (Variables|Default|GetTransitionCameraName) "Cave")
            (Default|ChangeCameratoCaveTeleport _ashero_character_bp)
            (goto _label)
            (else
              (Default|ChangeCameratoExternalTowerCamera _ashero_character_bp)
              (Audio|PlaySound2D "/Game/levels/MusicSFX/SFX/Tower_-_Sfx_-_Teleporte.Tower_-_Sfx_-_Teleporte" 1.0 1.0 0.0 0 0))))))
    (Utilities|FlowControl|Delay 5.0)
    (Transformation|SetActorLocation OtherActor (Transformation|GetActorLocation (Variables|Default|GetDestination)) false true)
    (Utilities|FlowControl|Delay 1.0)
    (Default|ChangeCameratoFollowCamera _ashero_character_bp)))

(event EventTick
  (params (DeltaSeconds :type Float%20%28single-precision%29)))

(fn ConstructionScript)