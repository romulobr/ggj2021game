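; Hero character Blueprint that switches the player's view between tower, teleport and follow cameras and records challenge completion.
; One function per camera makes a timed view-target blend on player controller 0.
; Completing the forest or maze sets its flag, then CompleteChallenge shows the external tower camera and returns to the follow camera after a delay.
; Mountain and cave completion functions are empty stubs, and the other camera functions are not called here.
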(event Custom|CompleteChallenge
  (CallFunction|ChangeCameratoExternalTowerCamera)
  (Utilities|FlowControl|Delay 3.0)
  (CallFunction|ChangeCameratoFollowCamera))

(event EventBeginPlay
  (|CallParentFunction) ; This node is disabled and will not be called.\nDrag off pins to build functionality.
)

(event Collision|EventActorBeginOverlap
  (params (OtherActor :type Actor%20Object%20Reference))
  (|CallParentFunction OtherActor) ; This node is disabled and will not be called.\nDrag off pins to build functionality.
)

(event EventTick
  (params (DeltaSeconds :type Float%20%28single-precision%29))
  (|CallParentFunction DeltaSeconds) ; This node is disabled and will not be called.\nDrag off pins to build functionality.
)

(fn ConstructionScript
  (|CallParentFunction))

(fn ChangeCameratoExternalTowerCamera
  (Game|Player|SetViewTargetwithBlend (Game|GetPlayerController 0) (Variables|Default|GetExternalTowerCameraActor) 3.0 "VTBlend_Linear" 0.0 false))

(fn ChangeCameratoFollowCamera
  (Game|Player|SetViewTargetwithBlend (Game|GetPlayerController 0) (Components|GetOwner (Variables|Default|GetFollowCamera)) 3.0 "VTBlend_Linear" 0.0 false))

(fn ChangeCameratoMountainTeleport
  (Game|Player|SetViewTargetwithBlend (Game|GetPlayerController 0) (Variables|Default|GetMountainTeleportCameraActor) 3.0 "VTBlend_Linear" 0.0 false))

(fn ChangeCameratoMazeTeleport
  (Game|Player|SetViewTargetwithBlend (Game|GetPlayerController 0) (Variables|Default|GetMazeTeleportCameraActor) 3.0 "VTBlend_Linear" 0.0 false))

(fn ChangeCameratoForestTeleport
  (Game|Player|SetViewTargetwithBlend (Game|GetPlayerController 0) (Variables|Default|GetForestTeleportCameraActor) 3.0 "VTBlend_Linear" 0.0 false))

(fn ChangeCameratoCaveTeleport
  (Game|Player|SetViewTargetwithBlend (Game|GetPlayerController 0) (Variables|Default|GetCaveTeleportCameraActor) 3.0 "VTBlend_Linear" 0.0 false))

(fn ChangeCameratoInternalTowerCamera
  (Game|Player|SetViewTargetwithBlend (Game|GetPlayerController 0) (Variables|Default|GetInternalTowerCameraActor) 3.0 "VTBlend_Linear" 0.0 false))

(fn CompleteForest
  (Variables|Default|SetisForestComplete true)
  (CallFunction|CompleteChallenge))

(fn CompleteMaze
  (Variables|Default|SetisMazeComplete true)
  (CallFunction|CompleteChallenge self))

(fn CompleteMountain)

(fn CompleteCave)