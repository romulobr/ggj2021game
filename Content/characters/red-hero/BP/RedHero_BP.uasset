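; RedHero_BP is a wandering character that completes the player's forest objective once the player stays close long enough to befriend it.
; Tick issues AI moves to random nearby navigable points about every second.
; Player overlap with its sphere lights a point light and starts a friendship timer, which any end overlap resets.
; Past the time limit, it sets its AnimBP standing, waits briefly, calls CompleteForest on the hero, then destroys itself.
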(event OnComponentBeginOverlap(Sphere)
  (params (OverlappedComponent :type Primitive%20Component%20Object%20Reference) (OtherActor :type Actor%20Object%20Reference) (OtherComp :type Primitive%20Component%20Object%20Reference) (OtherBodyIndex :type Integer) (bFromSweep :type Boolean) (SweepResult :type Hit%20Result%20Structure%20%28by%20ref%29))
  (if (== (Game|GetPlayerCharacter 0) OtherActor)
    (CallFunction|StartCounting)))

(event OnComponentEndOverlap(Sphere)
  (params (OverlappedComponent :type Primitive%20Component%20Object%20Reference) (OtherActor :type Actor%20Object%20Reference) (OtherComp :type Primitive%20Component%20Object%20Reference) (OtherBodyIndex :type Integer))
  (CallFunction|StopCounting))

(event EventBeginPlay
  (bind _asred_hero_abp (Utilities|Casting|CastToRedHero_ABP (Components|SkeletalMesh|GetAnimInstance (Variables|Default|GetSkeletalMesh))))
  (Variables|/Game/characters/red-hero/BP/RedHero_ABP.RedHero_ABP_C|SetIsStanding _asred_hero_abp 0.0))

(event Collision|EventActorBeginOverlap
  (params (OtherActor :type Actor%20Object%20Reference)))

(event EventTick
  (params (DeltaSeconds :type Float%20%28single-precision%29))
  (bind _result (CallFunction|ShouldChangeDirection DeltaSeconds))
  (if (Variables|Default|GetIsCounting)
    (Variables|Default|SetFriendshipTime (+ (Variables|Default|GetFriendshipTime) DeltaSeconds))
    (if (> (Variables|Default|GetFriendshipTime) (Variables|Default|GetTimeLimit))
      (Variables|/Game/characters/red-hero/BP/RedHero_ABP.RedHero_ABP_C|SetIsStanding (stale EventBeginPlay _asred_hero_abp) 1.0)
      (Utilities|FlowControl|Delay 2.0)
      (bind _ashero_character_bp (Utilities|Casting|CastToheroCharacter_BP (Game|GetPlayerCharacter 0)))
      (Default|CompleteForest _ashero_character_bp)
      (CallFunction|Dissapear)
      (else
        (if _result :!label _label
          (AI|AIMoveTo self (.RandomLocation (Class|NavigationSystemV1|GetRandomPointinNavigableRadius (Pawn|GetNavAgentLocation self) 5e+02 0 0)) 0 5.0 false))))
    (else
      (goto _label))))

(fn ConstructionScript)

(fn StartCounting
  (Variables|Default|SetIsCounting true)
  (Rendering|Components|Light|SetIntensity (Variables|Default|GetPointLight) 1e+04))

(fn StopCounting
  (Variables|Default|SetIsCounting false)
  (Variables|Default|SetFriendshipTime 0.0)
  (Rendering|Components|Light|SetIntensity (Variables|Default|GetPointLight) 0.0))

(fn Dissapear
  (Actor|DestroyActor))

(fn ShouldChangeDirection
  (params (DeltaTime :type Float%20%28single-precision%29))
  (bind _output_get (Variables|Default|SetDirectionTimeCounter (+ DeltaTime (Variables|Default|GetDirectionTimeCounter))))
  (if (> _output_get 1.0)
    (Variables|Default|SetDirectionTimeCounter 0.0)
    (return true)
    (else
      (return false))))