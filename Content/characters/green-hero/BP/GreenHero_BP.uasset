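; GreenHero_BP is a character the player befriends by staying nearby, which completes the maze.
; Player overlap with its Sphere lights a PointLight and starts a timer on Tick; any end overlap resets both.
; Past the time limit, it changes IsStanding on its anim Blueprint, waits briefly, then calls CompleteMaze on the player character.
; It then disappears by relocating its mesh and sphere rather than being destroyed.
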(event OnComponentBeginOverlap(Sphere)
  (params (OverlappedComponent :type Primitive%20Component%20Object%20Reference) (OtherActor :type Actor%20Object%20Reference) (OtherComp :type Primitive%20Component%20Object%20Reference) (OtherBodyIndex :type Integer) (bFromSweep :type Boolean) (SweepResult :type Hit%20Result%20Structure%20%28by%20ref%29))
  (if (== (Game|GetPlayerCharacter 0) OtherActor)
    (CallFunction|StartCounting)))

(event OnComponentEndOverlap(Sphere)
  (params (OverlappedComponent :type Primitive%20Component%20Object%20Reference) (OtherActor :type Actor%20Object%20Reference) (OtherComp :type Primitive%20Component%20Object%20Reference) (OtherBodyIndex :type Integer))
  (CallFunction|StopCounting))

(event EventBeginPlay
  (bind _asgreen_hero_abp (Utilities|Casting|CastToGreenHero_ABP (Components|SkeletalMesh|GetAnimInstance (Variables|Default|GetSkeletalMesh))))
  (Variables|/Game/characters/green-hero/BP/GreenHero_ABP.GreenHero_ABP_C|SetIsStanding _asgreen_hero_abp 0.0))

(event Collision|EventActorBeginOverlap
  (params (OtherActor :type Actor%20Object%20Reference)))

(event EventTick
  (params (DeltaSeconds :type Float%20%28single-precision%29))
  (if (Variables|Default|GetIsCounting)
    (Variables|Default|SetFriendshipTime (+ (Variables|Default|GetFriendshipTime) DeltaSeconds))
    (if (> (Variables|Default|GetFriendshipTime) (Variables|Default|GetTimeLimit))
      (Variables|/Game/characters/green-hero/BP/GreenHero_ABP.GreenHero_ABP_C|SetIsStanding (stale EventBeginPlay _asgreen_hero_abp) 5.0)
      (Utilities|FlowControl|Delay 2.0)
      (bind _ashero_character_bp (Utilities|Casting|CastToheroCharacter_BP (Game|GetPlayerCharacter 0)))
      (Default|CompleteMaze _ashero_character_bp)
      (CallFunction|Dissapear))))

(fn ConstructionScript)

(fn StartCounting
  (Variables|Default|SetIsCounting true)
  (Rendering|Components|Light|SetIntensity (Variables|Default|GetPointLight) 1e+04))

(fn StopCounting
  (Variables|Default|SetIsCounting false)
  (Variables|Default|SetFriendshipTime 0.0)
  (Rendering|Components|Light|SetIntensity (Variables|Default|GetPointLight) 0.0))

(fn Dissapear
  (Transformation|SetWorldLocation (Variables|Default|GetSkeletalMesh) "-100.000000,-100.000000,-100.000000" false false))